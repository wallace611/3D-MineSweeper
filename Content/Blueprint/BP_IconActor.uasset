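; BP_IconActor is an actor that displays numbered icons through eight components named 1 to 8.
; On BeginPlay, AddComponents collects those components in order into the Components array.
; ShowNumberIcon uses Val directly as an array index and makes that component visible, without propagating to children or hiding the others.
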(event EventBeginPlay
  (CallFunction|AddComponents))

(event EventShowNumberIcon
  (params (val :type Integer%20%28by%20ref%29))
  (Rendering|SetVisibility (Utilities|Array|Get(acopy) (Variables|Default|GetComponents) val) true false))

(fn ConstructionScript)

(fn AddComponents
  (bind _components (Variables|Default|GetComponents))
  (Utilities|Array|Add _components (Variables|Default|Get1))
  (Utilities|Array|Add _components (Variables|Default|Get2))
  (Utilities|Array|Add _components (Variables|Default|Get3))
  (Utilities|Array|Add _components (Variables|Default|Get4))
  (Utilities|Array|Add _components (Variables|Default|Get5))
  (Utilities|Array|Add _components (Variables|Default|Get6))
  (Utilities|Array|Add _components (Variables|Default|Get7))
  (Utilities|Array|Add _components (Variables|Default|Get8)))
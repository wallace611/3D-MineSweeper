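; BP_GameController is a game controller Blueprint that manages the HUD and the pause menu.
; BeginPlay adds the HUD to the viewport and sets Game and UI input mode, targeting a PauseMenu variable it has not yet created.
; The ToggleMenu input and a same-named event share one toggle, creating a fresh menu above the HUD or removing it, tracked by MenuOpened.
; The toggle does not pause the game.
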(event Custom|ToggleMenu
  (if (Variables|Default|GetbMenuOpened)
    (Widget|RemovefromParent (Variables|Default|GetPauseMenu))
    (Variables|Default|SetbMenuOpened false)
    (else
      (bind _returnvalue (UserInterface|CreateWidget "/Game/UI/PauseMenu.PauseMenu_C"))
      (bind _output_get (Variables|Default|SetPauseMenu _returnvalue))
      (UserInterface|Viewport|AddtoViewport _output_get 100)
      (Variables|Default|SetbMenuOpened true))))

(event EventBeginPlay
  (bind _returnvalue (UserInterface|CreateWidget "/Game/UI/HUD.HUD_C"))
  (UserInterface|Viewport|AddtoViewport _returnvalue 0)
  (Input|SetInputModeGameandUI (Game|GetPlayerController 0) (Variables|Default|GetPauseMenu) "DoNotLock" true false))

(event Input|ActionEvents|InputActionToggleMenu
  (params (Key :type Key%20Structure :default "None"))
  (:Pressed
    (if (Variables|Default|GetbMenuOpened)
      (Widget|RemovefromParent (Variables|Default|GetPauseMenu))
      (Variables|Default|SetbMenuOpened false)
      (else
        (bind _returnvalue (UserInterface|CreateWidget "/Game/UI/PauseMenu.PauseMenu_C"))
        (bind _output_get (Variables|Default|SetPauseMenu _returnvalue))
        (UserInterface|Viewport|AddtoViewport _output_get 100)
        (Variables|Default|SetbMenuOpened true)))))

(fn ConstructionScript)